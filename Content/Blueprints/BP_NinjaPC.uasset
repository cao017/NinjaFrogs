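; BP_NinjaPC is a player controller that runs local two-player play with a shared camera and health widget.
; An input action spawns player 2 once with a default controller, while this controller forwards both players' jump inputs to their pawns.
; Tick keeps player 1's spring arm at the pawns' midpoint, recenters it if player 2 is absent or dead, and possesses player 2 if player 1 dies.
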(event Input|EnhancedActionEvents|EnhancedInputActionIA_P2Enter
  (params (ActionValue :type Boolean) (ElapsedSeconds :type Float%20%28double-precision%29) (TriggeredSeconds :type Float%20%28double-precision%29) (InputAction :type Input%20Action%20Object%20Reference :default "/Game/Blueprints/EnhancedInput/IA_P2Enter.IA_P2Enter"))
  (:Completed
    (Utilities|FlowControl|DoOnce false
      (:Completed
        (bind _returnvalue (Game|SpawnActorfromClass "/Game/Blueprints/BP_PlayerBase.BP_PlayerBase_C" (Math|Transform|MakeTransform "100.000000,0.000000,350.000000" "0, 0, 0" "1.000000,1.000000,1.000000") "AlwaysSpawn" "MultiplyWithRoot" 0 false 0))
        (bind _output_get (Variables|Default|SetPlayer2Pawn _returnvalue))
        (Variables|/Game/Blueprints/BP_PlayerBase.BP_PlayerBase_C|SetHealthWidgetRef (Variables|Default|GetPlayer2Pawn) (Variables|Default|GetHealthWidgetRef))
        (Pawn|SpawnDefaultController _output_get)))))

(event Input|EnhancedActionEvents|EnhancedInputActionIA_Jump
  (params (ActionValue :type Boolean) (ElapsedSeconds :type Float%20%28double-precision%29) (TriggeredSeconds :type Float%20%28double-precision%29) (InputAction :type Input%20Action%20Object%20Reference :default "/Game/Blueprints/EnhancedInput/IA_Jump.IA_Jump"))
  (bind _player1pawn (Variables|Default|GetPlayer1Pawn))
  (:Triggered
    (Default|AddJump _player1pawn))
  (:Completed
    (Default|StopJump _player1pawn)))

(event Input|EnhancedActionEvents|EnhancedInputActionIA_P2Jump
  (params (ActionValue :type Boolean) (ElapsedSeconds :type Float%20%28double-precision%29) (TriggeredSeconds :type Float%20%28double-precision%29) (InputAction :type Input%20Action%20Object%20Reference :default "/Game/Blueprints/EnhancedInput/IA_P2Jump.IA_P2Jump"))
  (bind _player2pawn (Variables|Default|GetPlayer2Pawn))
  ;[1 1 1] player 2 jump
  (:Triggered
    (Default|AddJump _player2pawn))
  (:Completed
    (Default|StopJump _player2pawn)))

(event EventBeginPlay
  (bind _returnvalue (UserInterface|CreateWidget "/Game/Blueprints/UI/WBP_PlayerHealth.WBP_PlayerHealth_C"))
  (bind _output_get (Variables|Default|SetHealthWidgetRef _returnvalue))
  (UserInterface|Viewport|AddtoViewport _output_get 0)
  (Variables|/Game/Blueprints/BP_PlayerBase.BP_PlayerBase_C|SetHealthWidgetRef (Variables|Default|GetPlayer1Pawn) (Variables|Default|GetHealthWidgetRef))
  (Input|AddMappingContext (PlayerController|LocalPlayerSubsystems|GetEnhancedInputLocalPlayerSubsystem self) "/Game/Blueprints/EnhancedInput/NewInputMappingContext.NewInputMappingContext" 0 "(bIgnoreAllPressedKeysUntilRelease=True,bForceImmediately=False)"))

(event EventTick
  (params (DeltaSeconds :type Float%20%28single-precision%29))
  (Utilities|IsValid (Variables|Default|GetPlayer2Pawn)
    (:Is%20Valid
      (if (and (> (Variables|/Game/Blueprints/BP_PlayerBase.BP_PlayerBase_C|GetHealth (Variables|Default|GetPlayer2Pawn)) 0.0) (> (Variables|/Game/Blueprints/BP_PlayerBase.BP_PlayerBase_C|GetHealth (Variables|Default|GetPlayer1Pawn)) 0.0))
        (Transformation|SetWorldLocation (Variables|/Game/Blueprints/BP_PlayerBase.BP_PlayerBase_C|GetSpringArm (Variables|Default|GetPlayer1Pawn)) (/ (+ (Transformation|GetActorLocation (Variables|Default|GetPlayer1Pawn)) (Transformation|GetActorLocation (Variables|Default|GetPlayer2Pawn))) 2.0) false false)
        (elif (<= (Variables|/Game/Blueprints/BP_PlayerBase.BP_PlayerBase_C|GetHealth (Variables|Default|GetPlayer2Pawn)) 0.0)
          (Transformation|SetRelativeLocation (Variables|/Game/Blueprints/BP_PlayerBase.BP_PlayerBase_C|GetSpringArm (Variables|Default|GetPlayer1Pawn)) "0, 0, 0" false false)
          (elif (<= (Variables|/Game/Blueprints/BP_PlayerBase.BP_PlayerBase_C|GetHealth (Variables|Default|GetPlayer1Pawn)) 0.0)
            (Utilities|FlowControl|DoOnce false
              (:Completed
                (Pawn|Possess (Variables|Default|GetPlayer2Pawn))))))))
    (:Is%20Not%20Valid
      (Transformation|SetRelativeLocation (Variables|/Game/Blueprints/BP_PlayerBase.BP_PlayerBase_C|GetSpringArm (Variables|Default|GetPlayer1Pawn)) "0, 0, 0" false false))))

(event EventPossess
  (params (PossessedPawn :type Pawn%20Object%20Reference))
  (bind _asbp_player_base (Utilities|Casting|CastToBP_PlayerBase (Pawn|GetControlledPawn)))
  (Variables|Default|SetPlayer1Pawn _asbp_player_base))

(fn ConstructionScript)